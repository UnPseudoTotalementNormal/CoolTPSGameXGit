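; BP_BigTimer is an actor that shows a running elapsed-time clock in HH:MM:SS on a TextRender component.
; Tick feeds a one-second Delay, which ignores calls while pending, so the count advances about once a second and can drift with frame timing.
; Seconds roll over into minutes and minutes into hours, then ShowTime zero-pads each value and updates the text.
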(event EventBeginPlay)

(event Collision|EventActorBeginOverlap
  (params (OtherActor :type Actor%20Object%20Reference)))

(event EventTick
  (params (DeltaSeconds :type Float%20%28single-precision%29))
  (Utilities|FlowControl|Delay 1.0)
  (bind _output_get (Variables|Default|SetSeconds (+ (Variables|Default|GetSeconds) 1)))
  (if (>= _output_get 60)
    (Variables|Default|SetSeconds 0)
    (bind _output_get_2 (Variables|Default|SetMinutes (+ (Variables|Default|GetMinutes) 1)))
    (if (>= _output_get_2 60)
      (Variables|Default|SetMinutes 0)
      (Variables|Default|SetHours (+ (Variables|Default|GetHours) 1))))
  (CallFunction|ShowTime))

(fn ConstructionScript)

(fn ShowTime
  (bind _minutes (Variables|Default|GetMinutes))
  (bind _seconds (Variables|Default|GetSeconds))
  (bind _hours (Variables|Default|GetHours))
  (if (>= (Variables|Default|GetHours) 10)
    (Variables|Default|SetHoText (Utilities|String|ToString(Integer) _hours))
    (else
      (Variables|Default|SetHoText (Utilities|String|Append "0" (Utilities|String|ToString(Integer) _hours)))))
  (if (>= (Variables|Default|GetMinutes) 10)
    (Variables|Default|SetMinText (Utilities|String|ToString(Integer) _minutes))
    (else
      (Variables|Default|SetMinText (Utilities|String|Append "0" (Utilities|String|ToString(Integer) _minutes)))))
  (if (>= (Variables|Default|GetSeconds) 10)
    (Variables|Default|SetSecText (Utilities|String|ToString(Integer) _seconds))
    (else
      (Variables|Default|SetSecText (Utilities|String|Append "0" (Utilities|String|ToString(Integer) _seconds)))))
  (Rendering|Components|TextRender|SetText (Variables|Default|GetTextRender) (Utilities|Text|ToText(String) (Utilities|String|Append (Variables|Default|GetHoText) ":" (Variables|Default|GetMinText) ":" (Variables|Default|GetSecText)))))