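; BP_DialogueTrigger is a box trigger that shows dialogue text on the HUD when the player's BP_DolphinRagdoll overlaps it.
; It writes Text to the WHUD reached through BP_GameManager, then clears it after OnScreenTime.
; An optional ActivateQuest index of 0 also sets the manager's KrabyPaty flag.
; Triggered is set only after the delay, blocking later overlaps unless Retriggerable is on.
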(event OnComponentBeginOverlap(Box)
  (params (OverlappedComponent :type Primitive%20Component%20Object%20Reference) (OtherActor :type Actor%20Object%20Reference) (OtherComp :type Primitive%20Component%20Object%20Reference) (OtherBodyIndex :type Integer) (bFromSweep :type Boolean) (SweepResult :type Hit%20Result%20Structure%20%28by%20ref%29))
  (bind _activatequest (Variables|Default|GetActivateQuest))
  (if (Variables|Default|GetTriggered)
    (if (Variables|Default|GetRetriggerable)
      (Utilities|Casting|CastToBP_DolphinRagdoll OtherActor :!label _label)
      (bind _returnvalue (Actor|GetActorOfClass "/Game/Blueprints/BP_GameManager.BP_GameManager_C"))
      (Rendering|Components|TextRender|SetText (Variables|/Game/HUD/W_HUD.W_HUD_C|GetDialogueText (Variables|/Game/Blueprints/BP_GameManager.BP_GameManager_C|GetW%20HUD _returnvalue)) (Variables|Default|GetText))
      (if (!= _activatequest -1)
        (bind _returnvalue_2 (Actor|GetActorOfClass "/Game/Blueprints/BP_GameManager.BP_GameManager_C"))
        (switch int _activatequest
          (:Default
            _)
          (:0
            (Variables|/Game/Blueprints/BP_GameManager.BP_GameManager_C|SetKrabyPaty _returnvalue_2 true))))
      (Utilities|FlowControl|Delay (Variables|Default|GetOnScreenTime))
      (Rendering|Components|TextRender|SetText (Variables|/Game/HUD/W_HUD.W_HUD_C|GetDialogueText (Variables|/Game/Blueprints/BP_GameManager.BP_GameManager_C|GetW%20HUD _returnvalue)) "")
      (Variables|Default|SetTriggered true))
    (else
      (goto _label))))

(event EventBeginPlay)

(event EventTick
  (params (DeltaSeconds :type Float%20%28single-precision%29)))

(fn ConstructionScript)