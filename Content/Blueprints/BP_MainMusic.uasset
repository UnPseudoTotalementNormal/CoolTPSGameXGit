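; BP_MainMusic is the background music actor that switches tracks according to the boss event state.
; On BeginPlay it caches the BP_GameManager found in the level.
; Tick passes through a short Delay, throttling checks of the manager's BossEvent flag.
; Its Audio component gets PlinPlinPlon during a boss event and GoatSim otherwise, calling SetSound only when the track differs.
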(event EventBeginPlay
  (bind _returnvalue (Actor|GetActorOfClass "/Game/Blueprints/BP_GameManager.BP_GameManager_C"))
  (Variables|Default|SetGameManager _returnvalue))

(event Collision|EventActorBeginOverlap
  (params (OtherActor :type Actor%20Object%20Reference)))

(event EventTick
  (params (DeltaSeconds :type Float%20%28single-precision%29))
  (bind _audio (Variables|Default|GetAudio))
  (bind _sound (Variables|/Script/Engine.AudioComponent|GetSound _audio))
  (Utilities|FlowControl|Delay 0.2)
  (if (Variables|/Game/Blueprints/BP_GameManager.BP_GameManager_C|GetBossEvent (Variables|Default|GetGameManager))
    (if (!= _sound "/Game/Sounds/PlinPlinPlon.PlinPlinPlon")
      (Audio|Components|Audio|SetSound _audio "/Game/Sounds/PlinPlinPlon.PlinPlinPlon"))
    (elif (!= _sound "/Game/Sounds/GoatSim.GoatSim")
      (Audio|Components|Audio|SetSound _audio "/Game/Sounds/GoatSim.GoatSim"))))

(fn ConstructionScript)