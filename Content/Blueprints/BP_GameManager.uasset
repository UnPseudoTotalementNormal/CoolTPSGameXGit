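; Game manager that tracks the pirate-kill quest and shows its progress on the HUD.
; On BeginPlay it counts the P_PirateBoat actors in the level as the kill target.
; Tick uses a flag and a 0.2-second Delay to throttle text refreshes, looking up the W_HUD widget during the wait.
; The quest line shows DeadBoats against that total; DeadBoats is only read here.
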(event EventBeginPlay
  (bind _outactors (Actor|GetAllActorsOfClass "/Game/Boat/Boat/P_PirateBoat.P_PirateBoat_C"))
  (for _array_element _outactors
    (Variables|Default|SetBoatCounts (+ (Variables|Default|GetBoatCounts) 1))))

(event Collision|EventActorBeginOverlap
  (params (OtherActor :type Actor%20Object%20Reference)))

(event EventTick
  (params (DeltaSeconds :type Float%20%28single-precision%29))
  (if (Variables|Default|GetWaitingRefreshQuest)
    (if (== (Variables|Default|GetW%20HUD) 0)
      (bind _foundwidgets (Widget|GetAllWidgetsOfClass "/Game/HUD/W_HUD.W_HUD_C" true))
      (for _array_element _foundwidgets
        (Variables|Default|SetW%20HUD _array_element)))
    (else
      (Variables|Default|SetWaitingRefreshQuest true)
      (CallFunction|UpdatePirateKills)
      (Utilities|FlowControl|Delay 0.2)
      (Variables|Default|SetWaitingRefreshQuest false))))

(fn ConstructionScript)

(fn UpdatePirateKills
  (Rendering|Components|TextRender|SetText (Variables|/Game/HUD/W_HUD.W_HUD_C|GetPirateKills (Variables|Default|GetW%20HUD)) (Utilities|Text|ToText(String) (Utilities|String|Append "-Kill some pirates " (Utilities|String|ToString(Integer) (Variables|Default|GetDeadBoats)) "/" (Utilities|String|ToString(Integer) (Variables|Default|GetBoatCounts))))))